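; Base game mode Blueprint that shows the start and end screens of a match and toggles the player state.
; GameStart creates the start widget with the start delay, and GameOver creates the end widget with the win result.
; Both widgets receive the game mode as their parent before being added to the viewport.
; EnablePlayer and DisablePlayer are thin wrappers around EnablePlayerState and DisablePlayerState.
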(event EventGameStart
  (bind _returnvalue (UserInterface|CreateWidget "/Game/Blueprints/Widgets/WBP_GameStart.WBP_GameStart_C"))
  (Default|SetStartDelay _returnvalue (Variables|Default|GetStartDelay))
  (Default|SetParent _returnvalue self)
  (UserInterface|Viewport|AddtoViewport _returnvalue 0))

(event EventGameOver
  (params (PlayerWon :type Boolean))
  (bind _returnvalue (UserInterface|CreateWidget "/Game/Blueprints/Widgets/WBP_GameEnd.WBP_GameEnd_C"))
  (Default|SetPlayerWon _returnvalue PlayerWon)
  (Default|SetParent _returnvalue self)
  (UserInterface|Viewport|AddtoViewport _returnvalue 0))

(fn ConstructionScript)

(fn EnablePlayer
  (Class|TankGameModeBase|EnablePlayerState))

(fn DisablePlayer
  (Class|TankGameModeBase|DisablePlayerState))